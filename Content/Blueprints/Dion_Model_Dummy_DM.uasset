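; Destructible dummy target actor that awards score when a FlyingPawn hits it.
; When a FlyingPawn overlaps the Destructible component, it applies point damage to the hit actor from the sweep result, with the pawn as damage causer.
; A HitTarget flag makes the score bonus in BulletGameInstance apply only once, while damage is applied on every such overlap.
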(event `self.Destructible.OnComponentBeginOverlap`
  (params (OverlappedComponent :type "PrimitiveComponent Object Reference") (OtherActor :type "Actor Object Reference") (OtherComp :type "PrimitiveComponent Object Reference") (OtherBodyIndex :type Integer) (bFromSweep :type Boolean) (SweepResult :type "HitResult Structure (by ref)"))
  (bind (_bblockinghit _binitialoverlap _time _distance _location _impactpoint _normal _impactnormal _physmat _hitactor) (`GameplayStatics.BreakHitResult` SweepResult))
  (bind _asflying_pawn (cast `/Game/FlyingBP/Blueprints/FlyingPawn` OtherActor))
  (`GameplayStatics.ApplyPointDamage` _hitactor 100.0 _impactpoint SweepResult null _asflying_pawn)
  (if (not (`self.Hit Target`))
    (bind _asbullet_game_instance (cast `/Game/Blueprints/BulletGameInstance` (`GameplayStatics.GetGameInstance`)))
    (set `/Game/Blueprints/BulletGameInstance.Score` (+ (`/Game/Blueprints/BulletGameInstance.Score` _asbullet_game_instance) 100) _asbullet_game_instance)
    (set `self.Hit Target` true)))

(fn `UserConstructionScript`)